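; BP_PumpkinExplode is a fractured pumpkin actor that bursts apart as soon as play begins.
; The construction script gathers its ten pumpkin piece components into an array.
; BeginPlay enables physics on each piece and applies a one-time, mass-independent force based on the direction from an Arrow component to that piece.
; The multiplier zeroes X and Y, so the push is purely vertical.
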(event `self.ReceiveBeginPlay`
  (for _array_element (`self.Pieces`)
    (`PrimitiveComponent.SetSimulatePhysics` _array_element true)
    (`PrimitiveComponent.AddForce` _array_element (* (`KismetMathLibrary.Conv_RotatorToVector` (`KismetMathLibrary.FindLookAtRotation` (`SceneComponent.K2_GetComponentLocation` (`self.Arrow`)) (`SceneComponent.K2_GetComponentLocation` _array_element))) 500.0 (0.0 0.0 100.0)) "None" true)))

(fn `UserConstructionScript`
  (set `self.Pieces` (`|MakeArray` (`self.Pumpkin9`) (`self.Pumpkin3`) (`self.Pumpkin2`) (`self.Pumpkin1`) (`self.Pumpkin`) (`self.Pumpkin4`) (`self.Pumpkin8`) (`self.Pumpkin5`) (`self.Pumpkin7`) (`self.Pumpkin6`))))