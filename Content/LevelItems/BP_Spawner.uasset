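; Level-dressing spawner that scatters instanced copies of one of two meshes, chosen by Variation, over surfaces inside a box volume.
; The construction script sizes the box from ContentBox, then traces along the actor's down vector from random points in it, MeshCounter times.
; Each hit on the AttachToObj object types adds an instance with random yaw and scale.
; Placement is unseeded and has no runtime logic.
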(fn `UserConstructionScript`
  (bind (_origin _boxextent) (`KismetSystemLibrary.GetComponentBounds` (`self.Container`)))
  (bind _returnvalue (`KismetMathLibrary.MakeVector` (.x (`KismetMathLibrary.TransformLocation` (`self.GetTransform`) (`KismetMathLibrary.GreaterGreater_VectorRotator` (`KismetMathLibrary.InverseTransformLocation` (`self.GetTransform`) (`KismetMathLibrary.RandomPointInBoundingBox` _origin _boxextent)) (`self.K2_GetActorRotation`)))) (.y (`KismetMathLibrary.TransformLocation` (`self.GetTransform`) (`KismetMathLibrary.GreaterGreater_VectorRotator` (`KismetMathLibrary.InverseTransformLocation` (`self.GetTransform`) (`KismetMathLibrary.RandomPointInBoundingBox` _origin _boxextent)) (`self.K2_GetActorRotation`)))) (+ (.z (`KismetMathLibrary.TransformLocation` (`self.GetTransform`) (`KismetMathLibrary.GreaterGreater_VectorRotator` (`KismetMathLibrary.InverseTransformLocation` (`self.GetTransform`) (`KismetMathLibrary.RandomPointInBoundingBox` _origin _boxextent)) (`self.K2_GetActorRotation`)))) 100.0)))
  (`|ExecutionSequence`
    (:`then_0`
      (switch `int` (`self.Variation`)
        (:`0`
          (`StaticMeshComponent.SetStaticMesh` (`self.Mesh`) (`self.FirstMesh`))
          (`SceneComponent.K2_SetWorldRotation` :`self` (`self.Container`)))
        (:`1`
          (`StaticMeshComponent.SetStaticMesh` (`self.Mesh`) (`self.SecondMesh`)))))
    (:`then_1`
      (if (== (`self.ContentBox`) (0.0 0.0 0.0) :`ErrorTolerance` 0.0001)
        (set `self.ContentBox` (200.0 200.0 200.0)))
      (`BoxComponent.SetBoxExtent` (`self.Container`) (`self.ContentBox`) false)
      (for _ (range (`self.MeshCounter`))
        (bind (_outhit _returnvalue_2) (`KismetSystemLibrary.LineTraceSingleForObjects` _returnvalue (+ _returnvalue (* (* (`self.GetActorUpVector`) -1) 250.0)) (`self.AttachToObj`)))
        (if _returnvalue_2
          (`InstancedStaticMeshComponent.AddInstance` (`self.Mesh`) (`KismetMathLibrary.MakeTransform` (`.ImpactPoint` (`GameplayStatics.BreakHitResult` _outhit)) (`KismetMathLibrary.MakeRotator` 0.0 0.0 (`KismetMathLibrary.RandomFloatInRange` 0.0 (`self.MaxRotation`))) (`KismetMathLibrary.Conv_DoubleToVector` (+ (`KismetMathLibrary.RandomFloatInRange` (* (`self.RandomScale`) 1.0)) 1.0))) true))))))