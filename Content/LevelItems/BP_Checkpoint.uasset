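; BP_Checkpoint is a checkpoint level item that passes its Spawner transform to the player character on each overlap with its sphere.
; An inactive checkpoint also plays a sound and activation animation, then deactivates any other active checkpoint with a reverse animation, leaving one active.
; Every tick, the Checkpoint component smoothly yaws to track the player, using an interpolated look-at rotation with a 90-degree offset.
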(event `self.ReceiveTick`
  (params (DeltaSeconds :type "Float (single-precision)"))
  (bind _checkpoint (`self.Checkpoint`))
  (bind (_returnvalue_roll _returnvalue_pitch) (`KismetMathLibrary.BreakRotator` (`SceneComponent.K2_GetComponentRotation` _checkpoint)))
  (`/Engine/EditorBlueprintResources/StandardMacros.IsValid` (`GameplayStatics.GetPlayerCharacter` 0)
    (:`Is Valid`
      (`SceneComponent.K2_SetWorldRotation` _checkpoint (`KismetMathLibrary.MakeRotator` _returnvalue_roll _returnvalue_pitch (`self.LookAtZ`)) false false))))

(event `self.Sphere.OnComponentBeginOverlap`
  (params (OverlappedComponent :type "PrimitiveComponent Object Reference") (OtherActor :type "Actor Object Reference") (OtherComp :type "PrimitiveComponent Object Reference") (OtherBodyIndex :type Integer) (bFromSweep :type Boolean) (SweepResult :type "HitResult Structure (by ref)"))
  (bind _returnvalue (`GameplayStatics.GetPlayerCharacter` 0))
  (if (== OtherActor _returnvalue)
    (message `/Game/ThirdPerson/Blueprints/BPI_Pumpkin.SetCheckpoint` _returnvalue (`SceneComponent.K2_GetComponentToWorld` (`self.Spawner`)))
    (if (not (`self.Active`))
      (`GameplayStatics.PlaySoundAtLocation` "/Game/Audio/SC_Checkpoint.SC_Checkpoint" (`self.K2_GetActorLocation`) (struct) 1.0 1.0 0.0 null null null null)
      (`SkeletalMeshComponent.PlayAnimation` (`self.Checkpoint`) "/Game/Art/Checkpoint/AN_Checkpoint_Anim.AN_Checkpoint_Anim" false)
      (set `self.Active` true)
      (bind _outactors (`GameplayStatics.GetAllActorsOfClass` "BP_Checkpoint_C"))
      (for _array_element _outactors
        (if (!= _array_element self)
          (if (`/Game/LevelItems/BP_Checkpoint.Active` _array_element)
            (set `/Game/LevelItems/BP_Checkpoint.Active` false _array_element)
            (`SkeletalMeshComponent.PlayAnimation` (`/Game/LevelItems/BP_Checkpoint.Checkpoint` _array_element) "/Game/Art/Checkpoint/AN_Checkpoint_Reverse.AN_Checkpoint_Reverse" false)))))))

(fn `LookAtZ`
  (returns (ReturnValue :type "Float (double-precision)"))
  (bind (_returnvalue_roll _returnvalue_pitch _returnvalue_yaw) (`KismetMathLibrary.BreakRotator` (`SceneComponent.K2_GetComponentRotation` (`self.Checkpoint`))))
  (bind (_returnvalue_roll_2 _returnvalue_pitch_2 _returnvalue_yaw_2) (`KismetMathLibrary.BreakRotator` (`KismetMathLibrary.ComposeRotators` (`KismetMathLibrary.FindLookAtRotation` (`SceneComponent.K2_GetComponentLocation` (`self.Checkpoint`)) (`self.K2_GetActorLocation` (`GameplayStatics.GetPlayerCharacter` 0))) (struct :`Yaw` -90.0))))
  (return (`KismetMathLibrary.FInterpTo` _returnvalue_yaw _returnvalue_yaw_2 (`GameplayStatics.GetWorldDeltaSeconds`) 5.0)))

(fn `UserConstructionScript`)