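; BP_BlockWall is a Sky level obstacle that builds a wall of BP_PhantomPlatform blocks filling a box volume.
; The construction script sizes the Box from Bounds, and SpawnGrid divides its extent by Size to lay out rows, columns and layers.
; SpawnBlocks runs SpawnGrid, attaching each scaled platform to the Box in world space.
; DestroyBlocks clears the wall by destroying all attached actors, including nested ones.
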(event `SpawnBlocks`
  (`self.SpawnGrid`))

(event `DestroyBlocks`
  (for _array_element (`self.GetAttachedActors` true true)
    (`self.K2_DestroyActor` _array_element)))

(fn `SpawnGrid`
  (locals (BoxExtent :type "Vector Structure") (Origin :type "Vector Structure") (GridSize :type "Vector Structure") (StartPoints :type "Vector Structure") (Row :type Integer) (Column :type Integer))
  (bind (_startpoints_x _startpoints_y _startpoints_z) (`KismetMathLibrary.BreakVector` (`local.StartPoints`)))
  (bind _size (`self.Size`))
  (bind _size_2 (`self.Size`))
  (bind (_origin _boxextent) (`KismetSystemLibrary.GetComponentBounds` (`self.Box`)))
  (bind _returnvalue (* (`self.Size`) 2))
  (bind _returnvalue_2 (* _size -1))
  (bind _output_get (set `local.BoxExtent` _boxextent))
  (set `local.Origin` _origin)
  (bind _output_get_2 (set `local.GridSize` (`KismetMathLibrary.MakeVector` (/ (.x _output_get) _size_2) (/ (.y _output_get) _size_2) (/ (.z _output_get) _size_2))))
  (set `local.StartPoints` (- (`local.Origin`) (`local.BoxExtent`)))
  (bind _y (.y _output_get_2))
  (for _index (range 1 (+ (`KismetMathLibrary.FTrunc` (.z _output_get_2)) 1))
    (set `local.Row` 0)
    (set `local.Column` 0)
    (for _ (range 1 (+ (`KismetMathLibrary.FTrunc` (* (.x _output_get_2) _y)) 1))
      (if (> (`local.Column`) (- _y 1.0))
        (`/Engine/EditorBlueprintResources/StandardMacros.IncrementInt` (`local.Row`)
          (:`  `
            (set `local.Column` 1)))
        (else
          (`/Engine/EditorBlueprintResources/StandardMacros.IncrementInt` (`local.Column`)
            (:`  `
              _))))
      (bind _returnvalue_3 (`|SpawnActorFromClass` "/Game/LevelItems/Obstacles/3_Sky/BP_PhantomPlatform.BP_PhantomPlatform_C" (`KismetMathLibrary.MakeTransform` (`KismetMathLibrary.MakeVector` (+ (* (`local.Row`) _returnvalue) _startpoints_x (* _size 1)) (+ (* (`local.Column`) _returnvalue) _startpoints_y _returnvalue_2) (+ _startpoints_z (* _index _returnvalue) _returnvalue_2)) (struct) (2.0 2.0 2.0)) "AlwaysSpawn" "SelectDefaultAtRuntime" null null))
      (`self.K2_AttachToComponent` _returnvalue_3 (`self.Box`) "None" "KeepWorld" "KeepWorld" "KeepWorld" true))))

(fn `UserConstructionScript`
  (`BoxComponent.SetBoxExtent` (`self.Box`) (`self.Bounds`) false))