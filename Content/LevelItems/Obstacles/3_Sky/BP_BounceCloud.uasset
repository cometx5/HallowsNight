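; Sky-level obstacle cloud that bounces when the player touches it and can launch them on a jump press.
; Overlap plays a speed-scaled timeline that lerps the skeletal mesh between its construction-time location and an offset, re-arming through a Reset event.
; Jump input while overlapping launches the player using scaled Z displacement (previous minus current mesh position, sampled per qualifying press), only when that value is non-positive.
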(event `self.ReceiveBeginPlay`
  (bind _returnvalue (`GameplayStatics.GetPlayerController` 0))
  (bind _returnvalue_2 (pcsubsystem `EnhancedInputLocalPlayerSubsystem` _returnvalue))
  (set `self.NewLocation` (+ (`self.NewLocation`) (`self.InitialLocation`)))
  (`TimelineComponent.SetPlayRate` (`self.CloudBounce`) (`self.Speed`))
  (`/Engine/EditorBlueprintResources/StandardMacros.IsValid` _returnvalue_2
    (:`Is Valid`
      (`EnhancedInputSubsystemInterface.AddMappingContext` _returnvalue_2 "/Game/ThirdPerson/Input/IMC_Default.IMC_Default" 0 (struct))
      (`self.EnableInput` _returnvalue))))

(event `self.Collision.OnComponentBeginOverlap`
  (params (OverlappedComponent :type "PrimitiveComponent Object Reference") (OtherActor :type "Actor Object Reference") (OtherComp :type "PrimitiveComponent Object Reference") (OtherBodyIndex :type Integer) (bFromSweep :type Boolean) (SweepResult :type "HitResult Structure (by ref)"))
  (if (== OtherActor (`GameplayStatics.GetPlayerCharacter` 0))
    (`/Engine/EditorBlueprintResources/StandardMacros.DoOnce` false :!label _label
      (:`Completed`
        (bind (_direction _alpha) (`Timeline|CloudBounce` :!via `PlayFromStart`)
          (:`Update`
            (`SceneComponent.K2_SetWorldLocation` (`self.SkeletalMesh`) (`KismetMathLibrary.VLerp` (`self.InitialLocation`) (`self.NewLocation`) _alpha) false false))
          (:`Reset`
            (`self.ResetBounce`)))))))

(event `ResetBounce`
  (goto _label :!via `Reset`))

(event `EnhancedInput|/Game/ThirdPerson/Input/Actions/IA_Jump`
  (params (ActionValue :type Boolean) (ElapsedSeconds :type "Float (double-precision)") (TriggeredSeconds :type "Float (double-precision)") (InputAction :type "InputAction Object Reference" :default "/Game/ThirdPerson/Input/Actions/IA_Jump.IA_Jump"))
  (:`Started`
    (if (`KismetArrayLibrary.Array_Contains` (`PrimitiveComponent.GetOverlappingActors` (`self.Collision`) null) (`GameplayStatics.GetPlayerCharacter` 0))
      (bind _return (`self.Velocity`))
      (if (not (> (.z _return) 0.0))
        (`Character.LaunchCharacter` (`GameplayStatics.GetPlayerCharacter` 0) (`KismetMathLibrary.MakeVector` 0.0 0.0 (* (.z _return) 5.0)) false true)
        (`KismetSystemLibrary.PrintString` "Hello")))))

(fn `UserConstructionScript`
  (set `self.InitialLocation` (`self.K2_GetActorLocation`)))

(fn `Velocity`
  (returns (Return :type "Vector Structure"))
  (locals (Velocity :type "Vector Structure"))
  (set `local.Velocity` (- (`self.LastPosition`) (`SceneComponent.K2_GetComponentLocation` (`self.SkeletalMesh`))))
  (set `self.LastPosition` (`SceneComponent.K2_GetComponentLocation` (`self.SkeletalMesh`)))
  (return (`local.Velocity`)))