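; Phantom platform obstacle that vanishes after the player touches it, then returns once the player has left.
; Entering the Box trigger plays the Blink timeline on a dynamic material's Transparency, then disables collision.
; After a short delay it clears its Active lock and, unless the player still overlaps, runs FadeIn.
; FadeIn, also fired on exit when inactive, plays the Popback timeline and restores collision.
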(event `self.Box.OnComponentBeginOverlap`
  (params (OverlappedComponent :type "PrimitiveComponent Object Reference") (OtherActor :type "Actor Object Reference") (OtherComp :type "PrimitiveComponent Object Reference") (OtherBodyIndex :type Integer) (bFromSweep :type Boolean) (SweepResult :type "HitResult Structure (by ref)"))
  (if (== OtherActor (`GameplayStatics.GetPlayerCharacter` 0))
    (set `self.Colliding` true)
    (if (not (`self.Active`))
      (set `self.Active` true)
      (bind (_direction _blink) (`Timeline|Blink` :!via `PlayFromStart`)
        (:`Update`
          (`MaterialInstanceDynamic.SetScalarParameterValue` (`self.MatInst`) "Transparency" _blink))
        (:`Finished`
          (`PrimitiveComponent.SetCollisionEnabled` (`self.Collision`) "NoCollision")
          (`KismetSystemLibrary.Delay` 1.0)
          (set `self.Active` false)
          (if (not (`self.Colliding`))
            (`self.FadeIn`)))))))

(event `self.Box.OnComponentEndOverlap`
  (params (OverlappedComponent :type "PrimitiveComponent Object Reference") (OtherActor :type "Actor Object Reference") (OtherComp :type "PrimitiveComponent Object Reference") (OtherBodyIndex :type Integer))
  (if (== OtherActor (`GameplayStatics.GetPlayerCharacter` 0))
    (set `self.Colliding` false)
    (if (not (`self.Active`))
      (`self.FadeIn`))))

(event `FadeIn`
  (bind (_direction _blink) (`Timeline|Popback` :!via `PlayFromStart`)
    (:`Update`
      (`MaterialInstanceDynamic.SetScalarParameterValue` (`self.MatInst`) "Transparency" _blink))
    (:`Finished`
      (`PrimitiveComponent.SetCollisionEnabled` (`self.Collision`) "QueryAndPhysics")
      (set `self.Active` false))))

(fn `UserConstructionScript`
  (bind _returnvalue (`PrimitiveComponent.CreateDynamicMaterialInstance` (`self.Block`) 0 null "None"))
  (set `self.MatInst` _returnvalue))