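; Underground-level obstacle platform that flickers and vanishes after CH_PumpkinJuice steps on it, then returns.
; A DoOnce-guarded trigger plays an impact montage and Flicker timeline, whose Turn Off event hides both dynamic materials and lets pawns pass through.
; After a delay, ResetCollision restores visibility, blocking and the trigger, waiting until the character leaves the collision box if overlapping.
; The construction script sizes the boxes and SeeThrough from Size and creates the materials.
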(event `self.Trigger.OnComponentBeginOverlap`
  (params (OverlappedComponent :type "PrimitiveComponent Object Reference") (OtherActor :type "Actor Object Reference") (OtherComp :type "PrimitiveComponent Object Reference") (OtherBodyIndex :type Integer) (bFromSweep :type Boolean) (SweepResult :type "HitResult Structure (by ref)"))
  (cast `/Game/ThirdPerson/Blueprints/CH_PumpkinJuice` OtherActor)
  (`/Engine/EditorBlueprintResources/StandardMacros.DoOnce` false :!label _label
    (:`Completed`
      (set `self.Active` true)
      (`|ExecutionSequence`
        (:`then_0`
          (`|PlayMontage` (`self.Platform`) "/Game/Art/FallingPlatform/AM_FallingPlatform_Impact.AM_FallingPlatform_Impact"))
        (:`then_1`
          (bind (_direction _flicker) (`Timeline|Flicker` :!via `PlayFromStart`)
            (:`Update`
              (`MaterialInstanceDynamic.SetScalarParameterValue` (`self.Mat1`) "Flicker" _flicker)
              (`MaterialInstanceDynamic.SetScalarParameterValue` (`self.Mat2`) "Flicker" _flicker))
            (:`TurnOff`
              (`MaterialInstanceDynamic.SetScalarParameterValue` (`self.Mat1`) "Opacity" 0.0)
              (`MaterialInstanceDynamic.SetScalarParameterValue` (`self.Mat2`) "Opacity" 0.0)
              (`PrimitiveComponent.SetCollisionResponseToChannel` (`self.Collision`) "ECC_Pawn" "ECR_Overlap")
              (`PrimitiveComponent.SetCollisionResponseToChannel` (`self.Trigger`) "ECC_Pawn" "ECR_Ignore")
              (`KismetSystemLibrary.Delay` 2.0)
              (set `self.Active` false)
              (if (not (`self.Colliding`))
                (`self.ResetCollision`)))))))))

(event `ResetTrigger`
  (goto _label :!via `Reset`))

(event `self.Collision.OnComponentBeginOverlap`
  (params (OverlappedComponent :type "PrimitiveComponent Object Reference") (OtherActor :type "Actor Object Reference") (OtherComp :type "PrimitiveComponent Object Reference") (OtherBodyIndex :type Integer) (bFromSweep :type Boolean) (SweepResult :type "HitResult Structure (by ref)"))
  (cast `/Game/ThirdPerson/Blueprints/CH_PumpkinJuice` OtherActor)
  (set `self.Colliding` true))

(event `self.Collision.OnComponentEndOverlap`
  (params (OverlappedComponent :type "PrimitiveComponent Object Reference") (OtherActor :type "Actor Object Reference") (OtherComp :type "PrimitiveComponent Object Reference") (OtherBodyIndex :type Integer))
  (cast `/Game/ThirdPerson/Blueprints/CH_PumpkinJuice` OtherActor)
  (set `self.Colliding` false)
  (if (not (`self.Active`))
    (`self.ResetCollision`)))

(fn `ResetCollision`
  (`PrimitiveComponent.SetCollisionResponseToChannel` (`self.Collision`) "ECC_Pawn" "ECR_Block")
  (`PrimitiveComponent.SetCollisionResponseToChannel` (`self.Trigger`) "ECC_Pawn" "ECR_Overlap")
  (`self.ResetTrigger`)
  (`MaterialInstanceDynamic.SetScalarParameterValue` (`self.Mat1`) "Flicker" 0.0)
  (`MaterialInstanceDynamic.SetScalarParameterValue` (`self.Mat2`) "Flicker" 0.0)
  (`MaterialInstanceDynamic.SetScalarParameterValue` (`self.Mat1`) "Opacity" 1.0)
  (`MaterialInstanceDynamic.SetScalarParameterValue` (`self.Mat2`) "Opacity" 1.0))

(fn `UserConstructionScript`
  (bind _size (`self.Size`))
  (bind _platform (`self.Platform`))
  (bind (_returnvalue_x _returnvalue_y) (`KismetMathLibrary.BreakVector2D` (* _size 0.01)))
  (bind (_returnvalue_x_2 _returnvalue_y_2) (`KismetMathLibrary.BreakVector2D` (* _size 0.5)))
  (bind _returnvalue (+ _returnvalue_x_2 50.0))
  (`SceneComponent.SetWorldScale3D` (`self.SeeThrough`) (`KismetMathLibrary.MakeVector` (+ _returnvalue_x 1.2) (+ _returnvalue_y 1.2) 1.0))
  (`BoxComponent.SetBoxExtent` (`self.Collision`) (`KismetMathLibrary.MakeVector` _returnvalue (+ _returnvalue_y_2 50.0) 8.0) true)
  (`BoxComponent.SetBoxExtent` (`self.Trigger`) (`KismetMathLibrary.MakeVector` _returnvalue (+ _returnvalue_y_2 50.0) 8.0) true)
  (`PrimitiveComponent.SetBoundsScale` _platform _returnvalue)
  (`PrimitiveComponent.SetBoundsScale` (`self.Trigger`) _returnvalue)
  (bind _returnvalue_2 (`PrimitiveComponent.CreateDynamicMaterialInstance` _platform 0 null "None"))
  (set `self.Mat1` _returnvalue_2)
  (bind _returnvalue_3 (`PrimitiveComponent.CreateDynamicMaterialInstance` _platform 2 null "None"))
  (set `self.Mat2` _returnvalue_3))