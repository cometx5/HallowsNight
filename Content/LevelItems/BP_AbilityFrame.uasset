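; Ability pickup frame that unlocks its configured power when the player mashes Jump while inside its trigger sphere.
; Entering blends to the frame's view, swaps music for wind audio, glows and opens the spam widget.
; Taps fill a decaying meter driving pitch, spring-arm length, camera shake, Niagara and a spline-mesh soul trail tracking the player.
; Filling it disables the trigger and player input, shows the new-ability widget, then unlocks the power.
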(event `self.ReceiveBeginPlay`
  (bind _returnvalue (pcsubsystem `EnhancedInputLocalPlayerSubsystem` (`GameplayStatics.GetPlayerController` 0)))
  (bind _asw_spam_ability_button (cast `/Game/UI/Textures/W_SpamAbilityButton` (`WidgetComponent.GetWidget` (`self.SpamWidget`))))
  (bind _output_get (set `self.SpamRef` _asw_spam_ability_button))
  (set `/Game/UI/Textures/W_SpamAbilityButton.FrameRef` self _output_get)
  (bind _returnvalue_2 (`PrimitiveComponent.CreateDynamicMaterialInstance` (`self.SoulTrail`) 0 null "None"))
  (set `self.SoulTrailMatRef` _returnvalue_2)
  (`/Engine/EditorBlueprintResources/StandardMacros.IsValid` _returnvalue
    (:`Is Valid`
      (`EnhancedInputSubsystemInterface.AddMappingContext` _returnvalue "/Game/ThirdPerson/Input/IMC_Default.IMC_Default" 0 (struct)))))

(event `self.Sphere.OnComponentBeginOverlap`
  (params (OverlappedComponent :type "PrimitiveComponent Object Reference") (OtherActor :type "Actor Object Reference") (OtherComp :type "PrimitiveComponent Object Reference") (OtherBodyIndex :type Integer) (bFromSweep :type Boolean) (SweepResult :type "HitResult Structure (by ref)"))
  (bind _returnvalue (`GameplayStatics.GetPlayerCharacter` 0))
  (bind _returnvalue_2 (`GameplayStatics.GetPlayerController` 0))
  (bind _spamref (`self.SpamRef`))
  (if (== OtherActor _returnvalue)
    (if (not (`self.Completed`))
      (message `/Game/ThirdPerson/Blueprints/BPI_Pumpkin.InRangeOfFrame` _returnvalue true)
      (`self.Glow`)
      (set `self.Glowing` true)
      (`PlayerController.SetViewTargetWithBlend` (`GameplayStatics.GetPlayerController` 0) self 1.0 "VTBlend_Linear" 0.0 false)
      (bind _audio (`self.Audio`)
        (:`then`
          (`AudioComponent.FadeIn` _audio 1.0 1.0 0.0 "Linear"))
        (:`else`
          (bind _returnvalue_3 (`GameplayStatics.SpawnSound2D` "/Game/Audio/SC_BassWind.SC_BassWind" 1.0 1.0 0.0 null))
          (set `self.Audio` _returnvalue_3)))
      (message `/Game/ThirdPerson/Blueprints/BPI_Pumpkin.FadeOutMusic` _returnvalue_2 0.5)
      (`self.EnableInput` _returnvalue_2)
      (`UserWidget.PlayAnimation` _spamref (`/Game/UI/Textures/W_SpamAbilityButton.Open` _spamref) 0.0 1 "Forward" 1.0 false))))

(event `self.Sphere.OnComponentEndOverlap`
  (params (OverlappedComponent :type "PrimitiveComponent Object Reference") (OtherActor :type "Actor Object Reference") (OtherComp :type "PrimitiveComponent Object Reference") (OtherBodyIndex :type Integer))
  (bind _returnvalue (`GameplayStatics.GetPlayerCharacter` 0))
  (bind _spamref (`self.SpamRef`))
  (if (== OtherActor _returnvalue)
    (message `/Game/ThirdPerson/Blueprints/BPI_Pumpkin.InRangeOfFrame` _returnvalue true)
    (if (not (`self.Completed`))
      (`self.Unglow`)
      (set `self.Glowing` false)
      (`ActorComponent.Deactivate` (`self.NS_Frame`) :!label _label)
      (bind _shake (`self.Shake`)
        (:`then`
          (`PlayerCameraManager.StopCameraShake` (`GameplayStatics.GetPlayerCameraManager` 0) _shake true)
          (set `self.Shake` null))
        (:`else`
          _))
      (bind _returnvalue_2 (`GameplayStatics.GetActorOfClass` "/Game/LevelItems/Camera/BP_LevelCamera.BP_LevelCamera_C"))
      (`PlayerController.SetViewTargetWithBlend` (`GameplayStatics.GetPlayerController` 0) _returnvalue_2 1.0 "VTBlend_Linear" 0.0 false)
      (`AudioComponent.FadeOut` (`self.Audio`) 1.0 0.0 "Linear")
      (`self.DisableInput` (`GameplayStatics.GetPlayerController` 0))
      (`UserWidget.PlayAnimation` _spamref (`/Game/UI/Textures/W_SpamAbilityButton.Open` _spamref) 0.0 1 "Reverse" 1.0 false)
      (`KismetSystemLibrary.Delay` 0.5)
      (message `/Game/ThirdPerson/Blueprints/BPI_Pumpkin.FadeInMusic` (`GameplayStatics.GetPlayerController` 0) 2.0))))

(event `DeactivateEffects`
  (goto _label))

(event `Glow`
  (bind (_direction _glowy) (`Timeline|StartGlow` :!label _label_2)
    (:`Update`
      (`MaterialInstanceDynamic.SetScalarParameterValue` (`self.FrameMat`) "Glow" _glowy)
      (if (not (`self.Completed`))
        (`MaterialInstanceDynamic.SetScalarParameterValue` (`self.SoulTrailMatRef`) "Opacity" _glowy)))))

(event `Unglow`
  (goto _label_2 :!via `Reverse`))

(event `EnhancedInput|/Game/ThirdPerson/Input/Actions/IA_Jump`
  (params (ActionValue :type Boolean) (ElapsedSeconds :type "Float (double-precision)") (TriggeredSeconds :type "Float (double-precision)") (InputAction :type "InputAction Object Reference" :default "/Game/ThirdPerson/Input/Actions/IA_Jump.IA_Jump"))
  (bind _spamref (`self.SpamRef`))
  (bind _spamref_2 (`self.SpamRef`))
  (:`Started`
    (if (not (`self.Completed`))
      (set `self.Spam` (+ (`self.Spam`) (`KismetMathLibrary.RandomFloatInRange` 5.0 10.0)))
      (`/Game/UI/Textures/W_SpamAbilityButton.TapAnim` _spamref_2)
      (`Widget.SetRenderTransformAngle` (`/Game/UI/Textures/W_SpamAbilityButton.Flash` _spamref_2) (`KismetMathLibrary.RandomFloatInRange` -360.0 360.0))
      (`GameplayStatics.PlaySound2D` "/Game/Audio/SC_PianoG.SC_PianoG" 0.8 (`KismetMathLibrary.Lerp` 0.8 1.5 (`KismetMathLibrary.NormalizeToRange` (`self.Spam`) 0.0 100.0)) 0.0 null null)
      (if (> (`self.Spam`) 100.0)
        (set `self.Completed` true)
        (`GameplayStatics.PlaySound2D` "/Game/Audio/ahhhh-37191.ahhhh-37191" 1.2 1.0 0.0 null null)
        (`UserWidget.PlayAnimation` _spamref (`/Game/UI/Textures/W_SpamAbilityButton.Open` _spamref) 0.0 1 "Reverse" 1.0 false)
        (`AudioComponent.FadeOut` (`self.Audio`) 1.0 0.0 "Linear")
        (set `PrimitiveComponent.bGenerateOverlapEvents` false (`self.Sphere`))
        (`self.DisableInput` (`GameplayStatics.GetPlayerCharacter` 0) (`GameplayStatics.GetPlayerController` 0))
        (bind _returnvalue (`|CreateWidget` "/Game/UI/HUD/Frames/W_NewAbility_Sticky.W_NewAbility_Sticky_C"))
        (`UserWidget.AddToViewport` _returnvalue 0)
        (`KismetSystemLibrary.Delay` 3.0)
        (`self.DeactivateEffects`)
        (`MaterialInstanceDynamic.SetScalarParameterValue` (`self.SoulTrailMatRef`) "Opacity" 0.0)
        (message `/Game/ThirdPerson/Blueprints/BPI_Pumpkin.UnlockPower` (`GameplayStatics.GetPlayerCharacter` 0) (`self.Ability`))))))

(event `self.ReceiveTick`
  (params (DeltaSeconds :type "Float (single-precision)"))
  (bind _ns_frame (`self.NS_Frame`))
  (bind _spline (`self.Spline`))
  (`self.SpamEffects`)
  (`self.DetractSpam`)
  (`self.RotateSpamWidget` false)
  (if (`self.Glowing`)
    (`SceneComponent.K2_SetWorldLocation` _ns_frame (`KismetMathLibrary.VInterpTo` (`SceneComponent.K2_GetComponentLocation` _ns_frame) (`self.K2_GetActorLocation` (`GameplayStatics.GetPlayerCharacter` 0)) DeltaSeconds 10.0) false false)
    (`SplineComponent.SetLocationAtSplinePoint` (`self.Spline`) 1 (`self.K2_GetActorLocation` (`GameplayStatics.GetPlayerCharacter` 0)) "World" true)
    (`SplineMeshComponent.SetStartAndEnd` (`self.SoulTrail`) (`SplineComponent.GetLocationAtSplinePoint` _spline 0 "Local") (`SplineComponent.GetTangentAtSplinePoint` _spline 0 "Local") (`SplineComponent.GetLocationAtSplinePoint` _spline 1 "Local") (`SplineComponent.GetTangentAtSplinePoint` _spline 1 "Local") true)))

(fn `DetractSpam`
  (if (not (`self.Completed`))
    (set `self.Spam` (`KismetMathLibrary.FClamp` (- (`self.Spam`) (* 30.0 (`GameplayStatics.GetWorldDeltaSeconds`))) 0.0 100.0))))

(fn `RotateSpamWidget`
  (params (Debug :type Boolean))
  (bind _sphere1 (`self.Sphere1`))
  (bind _returnvalue (* (`GameplayStatics.GetWorldDeltaSeconds`) 100.0))
  (`SceneComponent.SetHiddenInGame` _sphere1 (not Debug) false)
  (`SceneComponent.SetHiddenInGame` (`self.Sphere2`) (not Debug) false)
  (`SceneComponent.SetHiddenInGame` (`self.Sphere3`) (not Debug) false)
  (`SceneComponent.K2_AddLocalRotation` _sphere1 (`KismetMathLibrary.MakeRotator` 0.0 _returnvalue) false false)
  (`SceneComponent.K2_AddLocalRotation` (`self.Sphere2`) (`KismetMathLibrary.MakeRotator` 0.0 (* _returnvalue -2.0)) false false))

(fn `SpamEffects`
  (bind _returnvalue (`GameplayStatics.GetPlayerCameraManager` 0))
  (bind _ns_frame (`self.NS_Frame`))
  (bind _soultrailmatref (`self.SoulTrailMatRef`))
  (if (not (`self.Completed`))
    (set `SpringArmComponent.TargetArmLength` (`KismetMathLibrary.Lerp` 100.0 -200.0 (`KismetMathLibrary.NormalizeToRange` (`self.Spam`) 0.0 100.0)) (`self.SpringArm`))
    (if (> (`self.Spam`) 15.0)
      (`self.Shake`
        (:`then`
          _)
        (:`else`
          (bind _returnvalue_2 (`LegacyCameraShake.StartLegacyCameraShake` _returnvalue "/Game/Art/CS_FrameMagic.CS_FrameMagic_C"))
          (set `self.Shake` _returnvalue_2)))
      (if (> (`self.Spam`) 30.0)
        (`ActorComponent.Activate` _ns_frame false)
        (bind _returnvalue_3 (`MaterialInstanceDynamic.K2_GetScalarParameterValue` _soultrailmatref "Spam"))
        (`MaterialInstanceDynamic.SetScalarParameterValue` _soultrailmatref "Spam" (`KismetMathLibrary.FInterpTo` _returnvalue_3 (`KismetMathLibrary.SelectFloat` 1.0 0.0 (> (`self.Spam`) 50.0)) (`GameplayStatics.GetWorldDeltaSeconds`) 10.0))
        (else
          (`ActorComponent.Deactivate` _ns_frame)))
      (else
        (bind _shake (`self.Shake`)
          (:`then`
            (`PlayerCameraManager.StopCameraShake` _returnvalue _shake true)
            (set `self.Shake` null))
          (:`else`))))))

(fn `UserConstructionScript`
  (bind _spline (`self.Spline`))
  (bind _returnvalue (`PrimitiveComponent.CreateDynamicMaterialInstance` (`self.Frame`) 0 null "None"))
  (set `self.FrameMat` _returnvalue)
  (bind _returnvalue_2 (`AddComponent|NODE_AddSplineMeshComponent-0`))
  (set `self.SoulTrail` _returnvalue_2)
  (`PrimitiveComponent.CreateDynamicMaterialInstance` _returnvalue_2 0 null "None")
  (`SceneComponent.K2_SetRelativeRotation` _returnvalue_2 (struct :`Yaw` 90.0) false false)
  (`SplineMeshComponent.SetStartAndEnd` _returnvalue_2 (`SplineComponent.GetLocationAtSplinePoint` _spline 0 "Local") (`SplineComponent.GetTangentAtSplinePoint` _spline 0 "Local") (`SplineComponent.GetLocationAtSplinePoint` _spline 1 "Local") (`SplineComponent.GetTangentAtSplinePoint` _spline 1 "Local") true)
  (`SceneComponent.SetRelativeScale3D` _returnvalue_2 (1.0 1.0 1.0))
  (`StaticMeshComponent.SetStaticMesh` _returnvalue_2 "/Game/Art/Frame/SM_Soul.SM_Soul"))