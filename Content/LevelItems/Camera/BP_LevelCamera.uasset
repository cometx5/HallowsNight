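; BP_LevelCamera is a level camera that becomes the view target on BeginPlay and follows the player along a spline.
; Each tick, the spring arm eases toward the spline point closest to the player and turns to that point's spline yaw.
; With a valid PointOfInterest, the camera also eases its rotation toward that actor or the spline yaw, depending on RotationMode.
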(event `self.ReceiveBeginPlay`
  (`PlayerController.SetViewTargetWithBlend` (`GameplayStatics.GetPlayerController` 0) self 0.0 "VTBlend_Linear" 0.0 false))

(event `self.ReceiveTick`
  (params (DeltaSeconds :type "Float (single-precision)"))
  (bind _springarm (`self.SpringArm`))
  (bind _camera (`self.Camera`))
  (bind (_returnvalue_roll _returnvalue_pitch _returnvalue_yaw) (`KismetMathLibrary.BreakRotator` (`KismetMathLibrary.Conv_VectorToRotator` (`SplineComponent.FindDirectionClosestToWorldLocation` (`self.Spline`) (`self.K2_GetActorLocation` (`GameplayStatics.GetPlayerCharacter` 0)) "World"))))
  (bind (_returnvalue_roll_2 _returnvalue_pitch_2 _returnvalue_yaw_2) (`KismetMathLibrary.BreakRotator` (`KismetMathLibrary.Conv_VectorToRotator` (`SplineComponent.FindDirectionClosestToWorldLocation` (`self.Spline`) (`self.K2_GetActorLocation` (`GameplayStatics.GetPlayerCharacter` 0)) "World"))))
  (`/Engine/EditorBlueprintResources/StandardMacros.IsValid` (`GameplayStatics.GetPlayerCharacter` 0)
    (:`Is Valid`
      (`SceneComponent.K2_SetWorldLocation` _springarm (`KismetMathLibrary.VInterpTo` (`SceneComponent.K2_GetComponentLocation` _springarm) (`SplineComponent.FindLocationClosestToWorldLocation` (`self.Spline`) (`self.K2_GetActorLocation` (`GameplayStatics.GetPlayerCharacter` 0)) "World") (`GameplayStatics.GetWorldDeltaSeconds`) 5.0) false false)
      (switch `/Game/LevelItems/Camera/E_CamStates` (`self.RotationMode`)
        (:`NewEnumerator0`
          _)
        (:`NewEnumerator2`
          _))
      (`SceneComponent.K2_SetWorldRotation` (`self.SpringArm`) (`KismetMathLibrary.RInterpTo` (`SceneComponent.K2_GetComponentRotation` (`self.SpringArm`)) (`KismetMathLibrary.MakeRotator` 0.0 0.0 _returnvalue_yaw) (`GameplayStatics.GetWorldDeltaSeconds`) (`self.CameraLagSpeed`)) false false)
      (`self.PointOfInterest`
        (:`then`
          (`SceneComponent.K2_SetWorldRotation` _camera (`KismetMathLibrary.RInterpTo` (`SceneComponent.K2_GetComponentRotation` _camera) (`KismetMathLibrary.SelectRotator` (`KismetMathLibrary.FindLookAtRotation` (`SceneComponent.K2_GetComponentLocation` (`self.Camera`)) (`self.K2_GetActorLocation` (`self.PointOfInterest`))) (`KismetMathLibrary.MakeRotator` 0.0 0.0 _returnvalue_yaw_2) (`|EnumEquality` (`self.RotationMode`) "NewEnumerator2")) (`GameplayStatics.GetWorldDeltaSeconds`) 1.0) false false))
        (:`else`)))))

(fn `UserConstructionScript`)