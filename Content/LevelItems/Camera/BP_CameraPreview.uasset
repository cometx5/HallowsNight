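; BP_CameraPreview previews the level camera on BP_LevelCamera's spline and precomputes its path.
; The construction script snaps it to the spline and poses the camera's spring arm from CameraStats.
; On BeginPlay it steps along the spline one unit at a time, storing locations and rotations.
; Sphere traces detect BP_CameraStateChange actors, exchange preview info and start distance-based yaw blends; otherwise rotation follows the current rotation mode.
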(event `self.ReceiveBeginPlay`
  (`self.BakeCameraInfo`)
  (bind _returnvalue (`GameplayStatics.GetActorOfClass` "/Game/LevelItems/Camera/BP_LevelCamera.BP_LevelCamera_C"))
  (set `self.CameraRef` _returnvalue))

(event `BakeCameraInfo`
  (bind _return (`self.LerpRotation`))
  (bind _transitioning (`self.Transitioning`))
  (bind _returnvalue (`GameplayStatics.GetActorOfClass` "/Game/LevelItems/Camera/BP_LevelCamera.BP_LevelCamera_C"))
  (bind _spline (`/Game/LevelItems/Camera/BP_LevelCamera.Spline` _returnvalue))
  (for _index (range (+ (`KismetMathLibrary.FTrunc` (`SplineComponent.GetSplineLength` _spline)) 1))
    (bind _returnvalue_2 (`SplineComponent.GetLocationAtDistanceAlongSpline` _spline (`KismetMathLibrary.Conv_IntToDouble` _index) "World"))
    (`self.K2_SetActorLocation` _returnvalue_2)
    (`KismetArrayLibrary.Array_Add` (`self.Locations`) _returnvalue_2)
    (`self.DetectTransitioner`)
    (if _transitioning
      (`self.K2_SetActorRotation` _return)
      (`KismetArrayLibrary.Array_Add` (`self.Rotations`) (`self.K2_GetActorRotation`))
      (else
        (`self.K2_SetActorRotation` (`KismetMathLibrary.SelectRotator` _return (`KismetMathLibrary.MakeRotator` 0.0 (`.PitchAdditive_10_58A3D6E24E5439D94FDA1997130B356D` (break `/Game/LevelItems/Camera/S_CamInfo` (`self.CameraStats`))) (.yaw (select `/Game/LevelItems/Camera/E_CamStates` (`.RotationMode_2_EB5ADD784F1FA97224AB9C99A4A6A781` (break `/Game/LevelItems/Camera/S_CamInfo` (`self.CameraStats`))) :`NewEnumerator0` (`SplineComponent.GetRotationAtDistanceAlongSpline` _spline (`KismetMathLibrary.Conv_IntToDouble` _index) "World") :`NewEnumerator1` (`self.K2_GetActorRotation`)))) _transitioning))
        (`KismetArrayLibrary.Array_Add` (`self.Rotations`) (`self.K2_GetActorRotation`))))))

(fn `DetectTransitioner`
  (bind _returnvalue (`self.K2_GetActorLocation`))
  (bind _outhit (`KismetSystemLibrary.SphereTraceSingle` _returnvalue _returnvalue 10.0 "TraceTypeQuery2"))
  (bind (_bblockinghit _binitialoverlap _time _distance _location _impactpoint _normal _impactnormal _physmat _hitactor) (`GameplayStatics.BreakHitResult` _outhit))
  (if _bblockinghit
    (bind _asbp_camera_state_change (cast `/Game/LevelItems/Camera/BP_CameraStateChange` _hitactor))
    (`/Game/LevelItems/Camera/BP_CameraStateChange.SetPreviewInfo` _asbp_camera_state_change (`self.CameraStats`))
    (if (and (`/Game/LevelItems/Camera/BP_CameraStateChange.Transition` _asbp_camera_state_change) (not (`self.Transitioning`)))
      (set `self.Transitioning` true)
      (bind _returnvalue_2 (`GameplayStatics.GetActorOfClass` "/Game/LevelItems/Camera/BP_LevelCamera.BP_LevelCamera_C"))
      (set `self.StartRotation` (`self.K2_GetActorRotation`))
      (bind _spline (`/Game/LevelItems/Camera/BP_LevelCamera.Spline` _returnvalue_2))
      (bind _returnvalue_3 (`SplineComponent.GetDistanceAlongSplineAtLocation` _spline (`self.K2_GetActorLocation`) "World"))
      (set `self.StartPoint` (`SplineComponent.GetLocationAtDistanceAlongSpline` _spline _returnvalue_3 "World"))
      (bind _returnvalue_4 (+ _returnvalue_3 (`self.TransitionDistance`)))
      (set `self.EndPoint` (`SplineComponent.GetLocationAtDistanceAlongSpline` _spline _returnvalue_4 "World"))
      (set `self.EndRotation` (`SplineComponent.GetRotationAtDistanceAlongSpline` _spline _returnvalue_4 "World")))))

(fn `LerpRotation`
  (returns (Return :type "Rotator Structure"))
  (locals (DistanceNormalized :type "Float (double-precision)"))
  (bind (_returnvalue_roll _returnvalue_pitch _returnvalue_yaw) (`KismetMathLibrary.BreakRotator` (`self.K2_GetActorRotation`)))
  (bind _endrotation (`self.EndRotation`))
  (bind _returnvalue (`GameplayStatics.GetActorOfClass` "/Game/LevelItems/Camera/BP_LevelCamera.BP_LevelCamera_C"))
  (set `self.CameraRef` _returnvalue)
  (if (`self.Transitioning`)
    (bind _output_get (set `self.TransitionPreviewDistance` (- (`SplineComponent.GetDistanceAlongSplineAtLocation` (`/Game/LevelItems/Camera/BP_LevelCamera.Spline` (`self.CameraRef`)) (`self.EndPoint`) "World") (`SplineComponent.GetDistanceAlongSplineAtLocation` (`/Game/LevelItems/Camera/BP_LevelCamera.Spline` (`self.CameraRef`)) (`self.StartPoint`) "World"))))
    (set `local.DistanceNormalized` (/ 1.0 _output_get))
    (if (`KismetMathLibrary.NearlyEqual_FloatFloat` _returnvalue_yaw (.yaw _endrotation) 0.1)
      (set `self.Transitioning` false)
      (else
        (return (`KismetMathLibrary.MakeRotator` 0.0 0.0 (.yaw (`KismetMathLibrary.RLerp` (`self.StartRotation`) _endrotation (* (- (`SplineComponent.GetDistanceAlongSplineAtLocation` (`/Game/LevelItems/Camera/BP_LevelCamera.Spline` (`self.CameraRef`)) (`self.K2_GetActorLocation`) "World") (`SplineComponent.GetDistanceAlongSplineAtLocation` (`/Game/LevelItems/Camera/BP_LevelCamera.Spline` (`self.CameraRef`)) (`self.StartPoint`) "World")) (`local.DistanceNormalized`)) true))))))))

(fn `PreviewDistanceFromPoint`
  (locals (CamRef :type "/Game/LevelItems/Camera/BP_LevelCamera Object Reference"))
  (bind _returnvalue (`GameplayStatics.GetActorOfClass` "/Game/LevelItems/Camera/BP_LevelCamera.BP_LevelCamera_C"))
  (bind _output_get (set `local.CamRef` _returnvalue))
  (bind _spline (`/Game/LevelItems/Camera/BP_LevelCamera.Spline` _output_get))
  (bind _returnvalue_2 (`SplineComponent.GetLocationAtDistanceAlongSpline` _spline (+ (`SplineComponent.GetDistanceAlongSplineAtLocation` _spline (`self.K2_GetActorLocation`) "World") (`self.TransitionPreviewDistance`)) "World"))
  (`KismetSystemLibrary.SphereTraceSingle` :`Start` _returnvalue_2 :`End` _returnvalue_2 :`Radius` 30.0 :`TraceChannel` "TraceTypeQuery1" :`DrawDebugType` "ForDuration" :`DrawTime` 10.0))

(fn `UserConstructionScript`
  (locals (CamRef :type "/Game/LevelItems/Camera/BP_LevelCamera Object Reference"))
  (bind _camref (`local.CamRef`))
  (bind _returnvalue (`GameplayStatics.GetActorOfClass` "/Game/LevelItems/Camera/BP_LevelCamera.BP_LevelCamera_C"))
  (bind _output_get (set `local.CamRef` _returnvalue))
  (bind _returnvalue_2 (`SplineComponent.FindLocationClosestToWorldLocation` (`/Game/LevelItems/Camera/BP_LevelCamera.Spline` _returnvalue) (`self.K2_GetActorLocation`) "World"))
  (`SceneComponent.K2_SetWorldLocation` (`/Game/LevelItems/Camera/BP_LevelCamera.SpringArm` _output_get) _returnvalue_2 false false)
  (`self.K2_SetActorLocation` _returnvalue_2)
  (set `SpringArmComponent.TargetOffset` (`KismetMathLibrary.MakeVector` 0.0 0.0 (`.TargetHeight_14_63FE0D0744FCD1F5DAB9CB86C963D749` (break `/Game/LevelItems/Camera/S_CamInfo` (`self.CameraStats`)))) (`/Game/LevelItems/Camera/BP_LevelCamera.SpringArm` _camref))
  (switch `/Game/LevelItems/Camera/E_CamStates` (`.RotationMode_2_EB5ADD784F1FA97224AB9C99A4A6A781` (break `/Game/LevelItems/Camera/S_CamInfo` (`self.CameraStats`)))
    (:`NewEnumerator0`
      (`SceneComponent.K2_SetWorldRotation` (`/Game/LevelItems/Camera/BP_LevelCamera.SpringArm` (`local.CamRef`)) (`KismetMathLibrary.MakeRotator` 0.0 (`.PitchAdditive_10_58A3D6E24E5439D94FDA1997130B356D` (break `/Game/LevelItems/Camera/S_CamInfo` (`self.CameraStats`))) (.yaw (`KismetMathLibrary.Conv_VectorToRotator` (`SplineComponent.FindDirectionClosestToWorldLocation` (`/Game/LevelItems/Camera/BP_LevelCamera.Spline` _camref) (`self.K2_GetActorLocation`) "World")))) false false))))