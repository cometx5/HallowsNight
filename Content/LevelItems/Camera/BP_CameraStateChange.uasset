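; BP_CameraStateChange is a level trigger box holding camera overrides: rotation mode, lag speed, pitch, target length and height.
; SetPreviewInfo writes these overrides into a passed-in CamInfo struct.
; The overlap event only casts to BP_CameraPreview, with nothing after it.
; Disconnected logic would store BP_LevelCamera's previous CamInfo and apply the overrides, adding a point of interest for one rotation mode.
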(event `self.Box.OnComponentBeginOverlap`
  (params (OverlappedComponent :type "PrimitiveComponent Object Reference") (OtherActor :type "Actor Object Reference") (OtherComp :type "PrimitiveComponent Object Reference") (OtherBodyIndex :type Integer) (bFromSweep :type Boolean) (SweepResult :type "HitResult Structure (by ref)"))
  (cast `/Game/LevelItems/Camera/BP_CameraPreview` OtherActor))

(fn `SetPreviewInfo`
  (params (StructRef :type "/Game/LevelItems/Camera/S_CamInfo Structure (by ref)"))
  (setmembers `/Game/LevelItems/Camera/S_CamInfo` :`StructRef` StructRef :`RotationMode` (`self.NewRotation Mode`) :`CameraLagSpeed` (`self.LagSpeed`) :`PitchAdditive` (`self.Pitch Additive`) :`TargetLength` (`self.Target Length`) :`TargetHeight` (`self.Target Height`)))

(fn `UserConstructionScript`)